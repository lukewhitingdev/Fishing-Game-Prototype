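; Interactable boat controls actor that lets a character in range take over piloting a boat.
; On BeginPlay it traces straight down on the Visibility channel and stores the boat character it hits as the attached boat.
; On interaction, the controller of the in-range character possesses that boat.
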(event `self.ReceiveBeginPlay`
  (bind (_returnvalue_x _returnvalue_y _returnvalue_z) (`KismetMathLibrary.BreakVector` (`self.K2_GetActorLocation`)))
  (`parent.ReceiveBeginPlay`)
  (bind (_outhit _returnvalue) (`KismetSystemLibrary.LineTraceSingle` (`self.K2_GetActorLocation`) (`KismetMathLibrary.MakeVector` _returnvalue_x _returnvalue_y (- _returnvalue_z 1000.0)) "TraceTypeQuery1"))
  (if _returnvalue
    (bind _asbp_boat_character (cast `/Game/Blueprints/BP_BoatCharacter` (`.HitActor` (`GameplayStatics.BreakHitResult` _outhit))))
    (set `self.AttachedBoat` _asbp_boat_character)))

(event `self.Interact_Blueprint`
  (bind _ascharacter (cast `Character` (`self.GetActorInRange`)))
  (`Controller.Possess` (`Pawn.GetController` _ascharacter) (`self.AttachedBoat`)))

(fn `UserConstructionScript`
  (`parent.UserConstructionScript`))